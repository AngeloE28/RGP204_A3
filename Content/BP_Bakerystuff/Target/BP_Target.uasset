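; BP_Target is a bread delivery target for the Kiki flight character in the bakery gameplay.
; When bread overlaps its cube, the bread moves back to the bakery target point for reuse, and the player's Seconds, carry state and Drop are triggered to reset the delivery.
; Any end overlap moves the target, after a short delay, to a random BP_TargetNewLocation actor using a hard-coded index range.
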(event OnComponentBeginOverlap(Cube)
  (params (OverlappedComponent :type Primitive%20Component%20Object%20Reference) (OtherActor :type Actor%20Object%20Reference) (OtherComp :type Primitive%20Component%20Object%20Reference) (OtherBodyIndex :type Integer) (bFromSweep :type Boolean) (SweepResult :type Hit%20Result%20Structure%20%28by%20ref%29))
  ;[1 1 1] Teleports the bread back to the baker instead of making a new one
  (bind _returnvalue (Actor|GetActorOfClass "/Game/BP_Bakerystuff/Bakery/BP_BakeryTargetPoint.BP_BakeryTargetPoint_C"))
  (bind _asbp_bread_pickup (Utilities|Casting|CastToBP_Bread_Pickup OtherActor))
  (Transformation|SetActorLocation _asbp_bread_pickup (Transformation|GetActorLocation _returnvalue) false false)
  (bind _asbp_my_kiki_flight (Utilities|Casting|CastToBP_MyKikiFlight (Game|GetPlayerCharacter 0)))
  (Variables|/Game/BP_Player/BP_MyKikiFlight.BP_MyKikiFlight_C|SetSeconds _asbp_my_kiki_flight 60)
  (Variables|/Game/BP_Player/BP_MyKikiFlight.BP_MyKikiFlight_C|SetPickedUp _asbp_my_kiki_flight false)
  (Default|Drop _asbp_my_kiki_flight))

(event OnComponentEndOverlap(Cube)
  (params (OverlappedComponent :type Primitive%20Component%20Object%20Reference) (OtherActor :type Actor%20Object%20Reference) (OtherComp :type Primitive%20Component%20Object%20Reference) (OtherBodyIndex :type Integer))
  ;[1 1 1] Teleports the target to a new location
  (bind _outactors (Actor|GetAllActorsOfClass "/Game/BP_Bakerystuff/Target/BP_TargetNewLocation.BP_TargetNewLocation_C"))
  (Utilities|FlowControl|Delay 1.0)
  (Transformation|SetActorLocation (Transformation|GetActorLocation (Utilities|Array|Get(acopy) _outactors (Math|Random|RandomIntegerinRange 0 12))) false false))

(fn ConstructionScript)