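; BP_Pointer is an actor that continuously rotates to point at a BP_Target actor in the level.
; Each Tick looks up a BP_Target, stores the reference and calls FaceTarget.
; FaceTarget smoothly interpolates the actor's rotation toward the target's location using look-at rotation and RInterpTo.
; It also re-calls itself after a very short Delay, forming a loop alongside the Tick-driven calls.
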(event Custom|FaceTarget
  ;[1 1 1] Face Target
  (Transformation|SetActorRotation (Math|Interpolation|RInterpTo (Transformation|GetActorRotation) (Math|Rotator|FindLookatRotation (Transformation|GetActorLocation) (Transformation|GetActorLocation (Variables|Default|GetBPTargetRef))) (Utilities|Time|GetWorldDeltaSeconds) 2e+01))
  (Utilities|FlowControl|Delay 0.001)
  (CallFunction|FaceTarget))

(event EventTick
  (params (DeltaSeconds :type Float%20%28single-precision%29))
  (bind _returnvalue (Actor|GetActorOfClass "/Game/BP_Bakerystuff/Target/BP_Target.BP_Target_C"))
  (Variables|Default|SetBPTargetRef _returnvalue)
  (CallFunction|FaceTarget))

(fn ConstructionScript)