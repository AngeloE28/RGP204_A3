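; BP_Aerial_Boost is a boost pickup that pushes the flying player character forward when it enters the trigger sphere.
; On overlap with player 0, it adds a velocity-change impulse along the character's forward vector through its CharacterMovement.
; The same overlap calls a PlaySound event that plays a whoosh sound at the player's location.
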(event OnComponentBeginOverlap(Sphere)
  (params (OverlappedComponent :type Primitive%20Component%20Object%20Reference) (OtherActor :type Actor%20Object%20Reference) (OtherComp :type Primitive%20Component%20Object%20Reference) (OtherBodyIndex :type Integer) (bFromSweep :type Boolean) (SweepResult :type Hit%20Result%20Structure%20%28by%20ref%29))
  ;[1 1 1] Boosting Forward event
  (if (== OtherActor (Game|GetPlayerCharacter 0))
    (CallFunction|PlaySound)
    (bind _askiki_flight (Utilities|Casting|CastToKikiFlight OtherActor))
    (Physics|AddImpulse (Variables|/Script/Engine.Character|GetCharacterMovement _askiki_flight) (* (Transformation|GetActorForwardVector _askiki_flight) 1e+03) true)))

(event Custom|Play%20Sound
  ;[1 1 1] Plays the sound effect
  (bind _asbp_my_kiki_flight (Utilities|Casting|CastToBP_MyKikiFlight (Game|GetPlayerCharacter 0)))
  (Audio|PlaySoundatLocation "/Game/Sounds/34172__glaneur-de-sons__woosh-02.34172__glaneur-de-sons__woosh-02" (Transformation|GetActorLocation _asbp_my_kiki_flight) "0, 0, 0" 1.0 1.0 0.0 0 0 0))

(event EventBeginPlay)

(event Collision|EventActorBeginOverlap
  (params (OtherActor :type Actor%20Object%20Reference)))

(event EventTick
  (params (DeltaSeconds :type Float%20%28single-precision%29)))

(fn ConstructionScript)