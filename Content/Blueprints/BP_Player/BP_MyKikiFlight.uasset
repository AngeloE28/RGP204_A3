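; Player Blueprint that carries physics objects, dropping them on a hit or bird flock overlap, and runs a game-over countdown.
; Left click toggles a camera line-trace grab through a PhysicsHandle, which follows GrabLocation each Tick while collision and damping change on the held object.
; The first pickup starts the countdown, paced by a Delay called from Tick, which pauses the game at zero.
; Pause and Resume manage the pause widget, input mode and cursor.
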(event OnComponentBeginOverlap(CapsuleComponent)
  (params (OverlappedComponent :type Primitive%20Component%20Object%20Reference) (OtherActor :type Actor%20Object%20Reference) (OtherComp :type Primitive%20Component%20Object%20Reference) (OtherBodyIndex :type Integer) (bFromSweep :type Boolean) (SweepResult :type Hit%20Result%20Structure%20%28by%20ref%29))
  ;[1 1 1] Player drops item when going through a bird flock
  (Utilities|Casting|CastToBP_BirdFlock OtherActor)
  (CallFunction|Drop))

(event Custom|Drop
  (bind _physicsobject (Variables|Default|GetPhysicsObject))
  ;[1 1 1] Drop Logic
  (Physics|Components|PhysicsHandle|ReleaseComponent (Variables|Default|GetPhysicsHandle))
  (Variables|Default|SetIsHoldingObject false)
  (Collision|SetCollisionResponsetoChannel _physicsobject "ECC_Pawn" "ECR_Block")
  (Class|PrimitiveComponent|SetAllPhysicsLinearVelocity _physicsobject "0, 0, 0" false)
  (Utilities|FlowControl|Delay 0.2)
  (Class|PrimitiveComponent|SetAngularDamping _physicsobject 0.0))

(event Custom|PickUp
  (bind _playercamera (Variables|Default|GetPlayerCamera))
  (bind _returnvalue (Transformation|GetWorldLocation _playercamera))
  ;[1 1 1] Pick up logic
  (bind (_outhit _returnvalue_2) (Collision|LineTraceForObjects _returnvalue (+ _returnvalue (* (Math|Vector|GetForwardVector _playercamera) 2e+03)) (Utilities|Array|MakeArray "ObjectTypeQuery4") false 0 "None"))
  (if _returnvalue_2
    (Variables|Default|SetPhysicsObject (.HitComponent (Collision|BreakHitResult _outhit)))
    (Class|PhysicsHandleComponent|GrabComponentatLocation (Variables|Default|GetPhysicsHandle) (.HitComponent (Collision|BreakHitResult _outhit)) "None" (.Location (Collision|BreakHitResult _outhit)))
    (Variables|Default|SetIsHoldingObject true)
    (Collision|SetCollisionResponsetoChannel (Variables|Default|GetPhysicsObject) "ECC_Pawn" "ECR_Ignore")
    (Class|PrimitiveComponent|SetAngularDamping (Variables|Default|GetPhysicsObject) 1e+01)
    (Variables|Default|SetPickedUp true)))

(event Custom|Timer
  ;[1 1 1] Count down timer
  (Utilities|FlowControl|Delay 1.0)
  (Variables|Default|SetSeconds (+ (Variables|Default|GetSeconds) -1))
  (if (== (Variables|Default|GetSeconds) 0)
    (Development|PrintString "Game Over! 
Out of Time!" true false "(R=1.000000,G=0.000000,B=0.004948,A=1.000000)")
    (Game|SetGamePaused true)))

(event EventBeginPlay)

(event Collision|EventActorBeginOverlap
  (params (OtherActor :type Actor%20Object%20Reference)))

(event EventTick
  (params (DeltaSeconds :type Float%20%28single-precision%29))
  ;[1 1 1] Set Handle Location
  (Physics|Components|PhysicsHandle|SetTargetLocation (Variables|Default|GetPhysicsHandle) (Transformation|GetWorldLocation (Variables|Default|GetGrabLocation)))
  (if (Variables|Default|GetPickedUp)
    (CallFunction|Timer)))

(event Collision|EventHit
  (params (MyComp :type Primitive%20Component%20Object%20Reference) (Other :type Actor%20Object%20Reference) (OtherComp :type Primitive%20Component%20Object%20Reference) (bSelfMoved :type Boolean) (HitLocation :type Vector :default "0, 0, 0") (HitNormal :type Vector :default "0, 0, 0") (NormalImpulse :type Vector :default "0, 0, 0") (Hit :type Hit%20Result%20Structure%20%28by%20ref%29))
  ;[1 1 1] Drops item on when player hits something
  (CallFunction|Drop))

(event Input|ActionEvents|InputActionPause
  (params (Key :type Key%20Structure :default "None"))
  ;[1 1 1] Pause the game with a pause menu
  (:Pressed
    (CallFunction|Pause)))

(event Input|MouseEvents|LeftMouseButton
  (params (Key :type Key%20Structure :default "None"))
  ;[1 1 1] Pick up and drop input
  (:Pressed
    (if (Variables|Default|GetIsHoldingObject)
      (CallFunction|Drop)
      (else
        (CallFunction|PickUp)))))

(fn ConstructionScript)

(fn Pause
  ;[1 1 1] Pauses the game with a pause menu
  (Game|SetGamePaused true)
  (Utilities|IsValid (Variables|Default|GetPauseMenu)
    (:Is%20Valid
      _)
    (:Is%20Not%20Valid
      (bind _returnvalue (UserInterface|CreateWidget "/Game/UI/PauseMenu.PauseMenu_C" (Game|GetPlayerController 0)))
      (Variables|Default|SetPauseMenu _returnvalue)))
  (UserInterface|Viewport|AddtoViewport (Variables|Default|GetPauseMenu) 0)
  (Input|SetInputModeUIOnly (Game|GetPlayerController 0) (Variables|Default|GetPauseMenu) "DoNotLock")
  (Variables|/Script/Engine.PlayerController|SetbShowMouseCursor (Game|GetPlayerController 0) true))

(fn Resume
  (bind _returnvalue (Game|GetPlayerController 0))
  ;[1 1 1] Resumes the game
  (Game|SetGamePaused false)
  (Widget|RemovefromParent (Variables|Default|GetPauseMenu))
  (Input|SetInputModeGameOnly _returnvalue)
  (Variables|/Script/Engine.PlayerController|SetbShowMouseCursor _returnvalue false))