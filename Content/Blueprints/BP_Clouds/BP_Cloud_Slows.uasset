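; BP_Cloud_Slows is a moving cloud obstacle that slows the player's flight character on contact.
; On begin play, a timeline, rated by Duration and started at CloudOffset, moves the cloud along the Track actor's spline, keeping its rotation.
; When Cloud_1 overlaps the player, it spawns a backward-facing effect, plays a sound and applies a backward velocity-change impulse to BP_MyKikiFlight.
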(event OnComponentBeginOverlap(Cloud_1)
  (params (OverlappedComponent :type Primitive%20Component%20Object%20Reference) (OtherActor :type Actor%20Object%20Reference) (OtherComp :type Primitive%20Component%20Object%20Reference) (OtherBodyIndex :type Integer) (bFromSweep :type Boolean) (SweepResult :type Hit%20Result%20Structure%20%28by%20ref%29))
  ;[1 1 1] Collision event
  (if (== OtherActor (Game|GetPlayerCharacter 0))
    (CallFunction|ActivateParticle)
    (CallFunction|PlaySound)
    (bind _asbp_my_kiki_flight (Utilities|Casting|CastToBP_MyKikiFlight OtherActor))
    (Physics|AddImpulse (Variables|/Script/Engine.Character|GetCharacterMovement _asbp_my_kiki_flight) (* (Transformation|GetActorForwardVector _asbp_my_kiki_flight) -1e+03) true)))

(event Custom|Move%20Clouds
  ;[1 1 1] Moves the clouds
  (Components|Timeline|SetPlayRate (Variables|Default|GetMoveCloud) (/ 1.0 (Variables|Default|GetDuration)))
  (Components|Timeline|SetNewTime (Variables|Default|GetMoveCloud) (Variables|Default|GetCloudOffset))
  (bind _alpha (Timeline|MoveCloud Play)
    (:Update
      (Variables|Default|SetAlpha _alpha)
      (Transformation|SetActorLocationAndRotation (Spline|GetLocationatDistanceAlongSpline (Variables|/Game/Blueprints/AI/BP_Track.BP_Track_C|GetTrackSpline (Variables|Default|GetTrack)) (Math|Float|Lerp 0.0 (Spline|GetSplineLength (Variables|/Game/Blueprints/AI/BP_Track.BP_Track_C|GetTrackSpline (Variables|Default|GetTrack))) (Variables|Default|GetAlpha)) "World") (Transformation|GetActorRotation)))))

(event Custom|Activate%20particle
  ;[1 1 1] Cloud effect
  (bind _asbp_my_kiki_flight (Utilities|Casting|CastToBP_MyKikiFlight (Game|GetPlayerCharacter 0)))
  (Niagara|SpawnSystematLocation "/Game/Blueprints/BP_Clouds/CloudEffectSystem.CloudEffectSystem" (Transformation|GetActorLocation _asbp_my_kiki_flight) (Math|Conversions|RotationFromXVector (* (Transformation|GetActorForwardVector _asbp_my_kiki_flight) -1.0))))

(event Custom|Play%20Sound
  ;[1 1 1] Plays the sound effect
  (bind _asbp_my_kiki_flight (Utilities|Casting|CastToBP_MyKikiFlight (Game|GetPlayerCharacter 0)))
  (Audio|PlaySoundatLocation "/Game/Sounds/34200__themfish__bamf.34200__themfish__bamf" (Transformation|GetActorLocation _asbp_my_kiki_flight) "0, 0, 0" 1.0 1.0 0.0 0 0 0))

(event EventBeginPlay
  ;[1 1 1] Starts the event
  (CallFunction|MoveClouds))

(event Collision|EventActorBeginOverlap
  (params (OtherActor :type Actor%20Object%20Reference)))

(event EventTick
  (params (DeltaSeconds :type Float%20%28single-precision%29)))

(fn ConstructionScript)