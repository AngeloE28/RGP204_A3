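; BP_Cloud_Slows_3 is a cloud obstacle that slows the player's flying Kiki character when they fly into it.
; When the player character begins overlapping the Cloud_3 component, it applies a backward velocity-change impulse along the character's forward vector to its CharacterMovement.
; The same overlap spawns a Niagara cloud effect at the player's location, oriented opposite to their facing direction.
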(event OnComponentBeginOverlap(Cloud_3)
  (params (OverlappedComponent :type Primitive%20Component%20Object%20Reference) (OtherActor :type Actor%20Object%20Reference) (OtherComp :type Primitive%20Component%20Object%20Reference) (OtherBodyIndex :type Integer) (bFromSweep :type Boolean) (SweepResult :type Hit%20Result%20Structure%20%28by%20ref%29))
  ;[1 1 1] Slowing down event
  (if (== OtherActor (Game|GetPlayerCharacter 0))
    (CallFunction|ActivateParticle)
    (bind _asbp_my_kiki_flight (Utilities|Casting|CastToBP_MyKikiFlight OtherActor))
    (Physics|AddImpulse (Variables|/Script/Engine.Character|GetCharacterMovement _asbp_my_kiki_flight) (* (Transformation|GetActorForwardVector _asbp_my_kiki_flight) -1e+03) true)))

(event Custom|Activate%20particle
  ;[1 1 1] Cloud effect
  (bind _asbp_my_kiki_flight (Utilities|Casting|CastToBP_MyKikiFlight (Game|GetPlayerCharacter 0)))
  (Niagara|SpawnSystematLocation "/Game/Blueprints/BP_Clouds/CloudEffectSystem.CloudEffectSystem" (Transformation|GetActorLocation _asbp_my_kiki_flight) (Math|Conversions|RotationFromXVector (* (Transformation|GetActorForwardVector _asbp_my_kiki_flight) -1.0))))

(event EventBeginPlay)

(event Collision|EventActorBeginOverlap
  (params (OtherActor :type Actor%20Object%20Reference)))

(event EventTick
  (params (DeltaSeconds :type Float%20%28single-precision%29)))

(fn ConstructionScript)