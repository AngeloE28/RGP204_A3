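; Yellow waving old man NPC that turns to face the BP_MyKikiFlight player when it comes within a set distance.
; Tick measures distance to the player's Kiki model, caching the player and starting FacePlayer in range, otherwise resetting rotation to zero after a tiny delay.
; FacePlayer smoothly interpolates toward a look-at rotation built from right-axis vectors.
; It re-calls itself through a short Delay with no exit condition, so turning continues once triggered.
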(event Custom|FacePlayer
  ;[1 1 1] Face Player
  (Transformation|SetActorRotation (Math|Conversions|RotationFromXVector (.Y (Math|Rotator|GetAxes (Math|Interpolation|RInterpTo (Math|Conversions|RotationFromXVector (.Y (Math|Rotator|GetAxes (Transformation|GetActorRotation)))) (Math|Conversions|RotationFromXVector (.Y (Math|Rotator|GetAxes (Math|Rotator|FindLookatRotation (Transformation|GetActorLocation) (Transformation|GetActorLocation (Variables|Default|GetPlayer)))))) (Utilities|Time|GetWorldDeltaSeconds) 2e+01)))))
  (Utilities|FlowControl|Delay 0.0001)
  (CallFunction|FacePlayer))

(event EventTick
  (params (DeltaSeconds :type Float%20%28single-precision%29))
  ;[1 1 1] Faces the player when player reaches a certain distance
  (if (< (Math|Vector|Distance(Vector) (Transformation|GetWorldLocation (Variables|SkeletalMeshActor|GetSkeletalMeshComponent)) (Transformation|GetWorldLocation (Variables|/Game/Blueprints/BP_Player/BP_MyKikiFlight.BP_MyKikiFlight_C|GetKiki_Model_Cat_In_The_Back (Variables|Default|GetPlayer)))) (Variables|Default|GetDistance))
    (bind _returnvalue (Actor|GetActorOfClass "/Game/Blueprints/BP_Player/BP_MyKikiFlight.BP_MyKikiFlight_C"))
    (Variables|Default|SetPlayer _returnvalue)
    (CallFunction|FacePlayer)
    (else
      (Utilities|FlowControl|Delay 0.0001)
      (Transformation|SetActorRotation "0, 0, 0"))))

(fn ConstructionScript)