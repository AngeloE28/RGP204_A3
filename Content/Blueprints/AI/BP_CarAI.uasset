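; BP_CarAI is an AI car actor that follows a track's spline.
; On BeginPlay, if ActiveCar is set, it plays the CarAIMover timeline with a play rate derived from Duration, starting at CarAIStartOffset.
; Each update maps the timeline Alpha to a distance along Track's spline, then sets the car's world location and rotation from that point, with no AI controller or pathfinding logic.
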(event Custom|MoveCarAI
  ;[1 1 1] AI follows a track
  (Components|Timeline|SetPlayRate (Variables|Default|GetCarAIMover) (/ 1.0 (Variables|Default|GetDuration)))
  (Components|Timeline|SetNewTime (Variables|Default|GetCarAIMover) (Variables|Default|GetCarAIStartOffset))
  (bind _alpha (Timeline|CarAIMover Play)
    (:Update
      (Variables|Default|SetAlpha _alpha)
      (Transformation|SetActorLocationAndRotation (Spline|GetLocationatDistanceAlongSpline (Variables|/Game/Blueprints/AI/BP_Track.BP_Track_C|GetTrackSpline (Variables|Default|GetTrack)) (Math|Float|Lerp 0.0 (Spline|GetSplineLength (Variables|/Game/Blueprints/AI/BP_Track.BP_Track_C|GetTrackSpline (Variables|Default|GetTrack))) (Variables|Default|GetAlpha)) "World") (Spline|GetRotationatDistanceAlongSpline (Variables|/Game/Blueprints/AI/BP_Track.BP_Track_C|GetTrackSpline (Variables|Default|GetTrack)) (Math|Float|Lerp 0.0 (Spline|GetSplineLength (Variables|/Game/Blueprints/AI/BP_Track.BP_Track_C|GetTrackSpline (Variables|Default|GetTrack))) (Variables|Default|GetAlpha)) "World")))))

(event EventBeginPlay
  ;[1 1 1] Starts the event
  (if (Variables|Default|GetActiveCar)
    (CallFunction|MoveCarAI)))

(event Collision|EventActorBeginOverlap
  (params (OtherActor :type Actor%20Object%20Reference)))

(event EventTick
  (params (DeltaSeconds :type Float%20%28single-precision%29)))

(fn ConstructionScript)